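; Turf is a grid tile actor for a tilemap, representing space, lattice, catwalk, plating, floor or wall.
; The construction script calls SetTileType, which swaps the static mesh, creates a dynamic material instance for non-empty types, and sets whether the tile is in space and can be entered.
; DiscoverNeighborTiles offsets its coordinate by each Neighbors key's delta and stores valid in-range turfs from the TileMap in that map.
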(fn `DiscoverNeighborTiles`
  (bind (_coord_x _coord_y) (break `/Game/Library/Coord` (`self.Coord`)))
  (bind _keys (`BlueprintMapLibrary.Map_Keys` (`self.Neighbors`)))
  (for _array_element _keys
    (bind _tilemap (`self.TileMap`)
      (:`then`
        (bind (_x _y) (break `/Game/Library/Coord` (`/Game/Directions/Direction.Delta` _array_element)))
        (bind _coord (make `/Game/Library/Coord` (+ _x _coord_x) (+ _y _coord_y)))
        (if (`/Game/Library/GridMath.IsCoordInRange` _tilemap _coord)
          (bind _turf (`/Game/Blueprints/BP_TileMap.GetTurfAtCoord` _tilemap _coord))
          (`/Engine/EditorBlueprintResources/StandardMacros.IsValid` _turf
            (:`Is Valid`
              (`BlueprintMapLibrary.Map_Add` (`self.Neighbors`) _array_element _turf)))))
      (:`else`))))

(fn `SetTileType`
  (params (TurfType :type Integer))
  (bind _output_get (set `self.TurfType` TurfType))
  (switch `int` _output_get
    (:`0`
      (set `self.isInSpace?` true)
      (set `self.CanEnter?` true)
      (`StaticMeshComponent.SetStaticMesh` (`self.StaticMesh`) null))
    (:`1`
      (`StaticMeshComponent.SetStaticMesh` (`self.StaticMesh`) (`self.LatticeSM`))
      (bind _returnvalue (`PrimitiveComponent.CreateDynamicMaterialInstance` (`self.StaticMesh`) 0 "/Game/Materials/MI_Catwalk.MI_Catwalk" "None"))
      (set `self.MaterialInstance` _returnvalue)
      (set `self.isInSpace?` true)
      (set `self.CanEnter?` true))
    (:`2`
      (`StaticMeshComponent.SetStaticMesh` (`self.StaticMesh`) (`self.CatwalkSM`))
      (bind _returnvalue_2 (`PrimitiveComponent.CreateDynamicMaterialInstance` (`self.StaticMesh`) 0 "/Game/StarterContent/Materials/M_Metal_Burnished_Steel.M_Metal_Burnished_Steel" "None"))
      (set `self.MaterialInstance` _returnvalue_2)
      (set `self.isInSpace?` true)
      (set `self.CanEnter?` true))
    (:`3`
      (`StaticMeshComponent.SetStaticMesh` (`self.StaticMesh`) (`self.PlatingSM`))
      (bind _returnvalue_3 (`PrimitiveComponent.CreateDynamicMaterialInstance` (`self.StaticMesh`) 0 "/Game/StarterContent/Materials/M_Concrete_Tiles.M_Concrete_Tiles" "None"))
      (set `self.MaterialInstance` _returnvalue_3)
      (set `self.isInSpace?` false)
      (set `self.CanEnter?` true))
    (:`4`
      (`StaticMeshComponent.SetStaticMesh` (`self.StaticMesh`) (`self.FloorSM`))
      (bind _returnvalue_4 (`PrimitiveComponent.CreateDynamicMaterialInstance` (`self.StaticMesh`) 0 "/Game/StarterContent/Materials/M_Ceramic_Tile_Checker.M_Ceramic_Tile_Checker" "None"))
      (set `self.MaterialInstance` _returnvalue_4)
      (set `self.isInSpace?` false)
      (set `self.CanEnter?` true))
    (:`5`
      (`StaticMeshComponent.SetStaticMesh` (`self.StaticMesh`) (`self.WallSM`))
      (bind _returnvalue_5 (`PrimitiveComponent.CreateDynamicMaterialInstance` (`self.StaticMesh`) 0 "/Game/Materials/MI_Walltile.MI_Walltile" "None"))
      (set `self.MaterialInstance` _returnvalue_5)
      (set `self.isInSpace?` false)
      (set `self.CanEnter?` false))))

(fn `UserConstructionScript`
  (`parent.UserConstructionScript`)
  (`self.SetTileType` (`self.TurfType`)))