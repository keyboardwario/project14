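; Turf is a map tile for space, lattice, catwalk, plating, floor or wall, with its own atmosphere.
; Construction sets mesh, dynamic material and space/density flags by type, then fills default air, temperature and pressure.
; It finds neighbors through the TileMap, and AirExchange pools gases with plating and floor neighbors, writing results back to those neighbors.
; A widget shows air values every tick, and AddDoor spawns an attached door.
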(event `self.ReceiveTick`
  (params (DeltaSeconds :type "Float (single-precision)"))
  (`self.UpdateAirHUD`))

(fn `AddDoor`
  (bind _returnvalue (`|SpawnActorFromClass` "/Game/Blueprints/Atom/Object/Machine/Door/Door.Door_C" (`self.GetTransform` self) "Undefined" "OverrideRootScale" null (`self.TileMap`) self null))
  (`KismetArrayLibrary.Array_AddUnique` (`self.Contents`) _returnvalue)
  (`self.K2_AttachToActor` _returnvalue self "None" "KeepRelative" "KeepRelative" "KeepRelative" true))

(fn `AirExchange`
  (locals (L_Oxygen :type Integer) (L_Nitrogen :type Integer) (L_Co2 :type Integer) (L_Temp :type Integer) (L_Pressure :type Integer) (L_NumExchangers :type Integer :default 0))
  (`/Engine/EditorBlueprintResources/StandardMacros.IsValid` (`|GetArrayItem` (`self.NeighborTurfsThatCanHaveAir`))
    (:`Is Valid`
      (`|ExecutionSequence`
        (:`then_0`
          (`|ExecutionSequence`
            (:`then_0`
              (set `local.L_Oxygen` (+ (`self.Oxygen`) (`local.L_Oxygen`))))
            (:`then_1`
              (set `local.L_Nitrogen` (+ (`self.Nitrogen`) (`local.L_Nitrogen`))))
            (:`then_2`
              (set `local.L_Co2` (+ (`self.CarbonDioxide`) (`local.L_Co2`))))))
        (:`then_1`
          (for _array_element (`self.NeighborTurfsThatCanHaveAir`)
            (`|ExecutionSequence`
              (:`then_0`
                (set `local.L_Oxygen` (+ (`local.L_Oxygen`) (`/Game/Blueprints/Turf/Turf.Oxygen` _array_element))))
              (:`then_1`
                (set `local.L_Nitrogen` (+ (`local.L_Nitrogen`) (`/Game/Blueprints/Turf/Turf.Nitrogen` _array_element))))
              (:`then_2`
                (set `local.L_Co2` (+ (`local.L_Co2`) (`/Game/Blueprints/Turf/Turf.CarbonDioxide` _array_element)))))))
        (:`then_2`
          (set `local.L_NumExchangers` (`KismetArrayLibrary.Array_Length` (`self.NeighborTurfsThatCanHaveAir`)))
          (`|ExecutionSequence`
            (:`then_0`
              (set `local.L_Oxygen` (/ (`local.L_Oxygen`) (`local.L_NumExchangers`))))
            (:`then_1`
              (set `local.L_Nitrogen` (/ (`local.L_Nitrogen`) (`local.L_NumExchangers`))))
            (:`then_2`
              (set `self.CarbonDioxide` (/ (`self.CarbonDioxide`) (`local.L_NumExchangers`))))))
        (:`then_3`
          (for _array_element_2 (`self.NeighborTurfsThatCanHaveAir`)
            (`self.SetAirAmounts` _array_element_2 (`local.L_Oxygen`) (`local.L_Nitrogen`) (`local.L_Co2`))))
        (:`then_4`
          (`self.UpdateAirHUD`))))))

(fn `ChangeTemperature`
  (set `self.Temperature` (+ (`self.DeltaTemperature`) (`self.Temperature`)))
  (set `self.DeltaTemperature` 0))

(fn `DefaultAir`
  (if (`self.isInSpace?`)
    (`self.SetAirAmounts` 0)
    (set `self.Temperature` 0)
    (set `self.Pressure` 0)
    (else
      (`self.SetAirAmounts` 18 80 2)
      (set `self.Temperature` 280)
      (set `self.Pressure` 101)))
  (`self.UpdateAirHUD`))

(fn `DiscoverNeighborTiles`
  (bind (_coord_x _coord_y) (break `/Game/Library/Coord` (`self.Coord`)))
  (bind _keys (`BlueprintMapLibrary.Map_Keys` (`self.Neighbors`)))
  (for _array_element _keys
    (bind _tilemap (`self.TileMap`)
      (:`then`
        (bind (_x _y) (break `/Game/Library/Coord` (`/Game/Directions/Direction.Delta` _array_element)))
        (bind _coord (make `/Game/Library/Coord` (+ _x _coord_x) (+ _y _coord_y)))
        (if (`/Game/Library/GridMath.IsCoordInRange` _tilemap _coord)
          (bind _turf (`/Game/Blueprints/BP_TileMap.GetTurfAtCoord` _tilemap _coord))
          (`/Engine/EditorBlueprintResources/StandardMacros.IsValid` _turf
            (:`Is Valid`
              (`BlueprintMapLibrary.Map_Add` (`self.Neighbors`) _array_element _turf)))))
      (:`else`))))

(fn `FindOpenAirNeighbors`
  (bind _neighbors (`self.Neighbors`))
  (bind _turftype (`self.TurfType`))
  (if (or (== _turftype 3) (== _turftype 4))
    (`KismetArrayLibrary.Array_Clear` (`self.NeighborTurfsThatCanHaveAir`))
    (bind _keys (`BlueprintMapLibrary.Map_Keys` _neighbors))
    (for _array_element _keys
      (bind _value (`BlueprintMapLibrary.Map_Find` _neighbors _array_element))
      (`/Engine/EditorBlueprintResources/StandardMacros.IsValid` _value
        (:`Is Valid`
          (bind _turftype_2 (`/Game/Blueprints/Turf/Turf.TurfType` _value))
          (if (or (== _turftype_2 3) (== _turftype_2 4))
            (`KismetArrayLibrary.Array_AddUnique` (`self.NeighborTurfsThatCanHaveAir`) _value)))))))

(fn `SetAirAmounts`
  (params (Oxygen :type Integer) (Nitrogen :type Integer) (CarbonDioxide :type Integer))
  (set `self.Oxygen` Oxygen)
  (set `self.Nitrogen` Nitrogen)
  (set `self.CarbonDioxide` CarbonDioxide)
  (`self.UpdateAirHUD`))

(fn `SetTileType`
  (params (TurfType :type Integer))
  (bind _output_get (set `self.TurfType` TurfType))
  (switch `int` _output_get
    (:`0`
      (set `self.isInSpace?` true)
      (set `self.IsDense?` false)
      (`StaticMeshComponent.SetStaticMesh` (`self.StaticMesh`) null))
    (:`1`
      (`StaticMeshComponent.SetStaticMesh` (`self.StaticMesh`) (`self.LatticeSM`))
      (bind _returnvalue (`PrimitiveComponent.CreateDynamicMaterialInstance` (`self.StaticMesh`) 0 "/Game/Materials/MI_Catwalk.MI_Catwalk" "None"))
      (set `self.MaterialInstance` _returnvalue)
      (set `self.isInSpace?` true)
      (set `self.IsDense?` false))
    (:`2`
      (`StaticMeshComponent.SetStaticMesh` (`self.StaticMesh`) (`self.CatwalkSM`))
      (bind _returnvalue_2 (`PrimitiveComponent.CreateDynamicMaterialInstance` (`self.StaticMesh`) 0 "/Game/StarterContent/Materials/M_Metal_Burnished_Steel.M_Metal_Burnished_Steel" "None"))
      (set `self.MaterialInstance` _returnvalue_2)
      (set `self.isInSpace?` true)
      (set `self.IsDense?` false))
    (:`3`
      (`StaticMeshComponent.SetStaticMesh` (`self.StaticMesh`) (`self.PlatingSM`))
      (bind _returnvalue_3 (`PrimitiveComponent.CreateDynamicMaterialInstance` (`self.StaticMesh`) 0 "/Game/StarterContent/Materials/M_Concrete_Tiles.M_Concrete_Tiles" "None"))
      (set `self.MaterialInstance` _returnvalue_3)
      (set `self.isInSpace?` false :!label _label)
      (set `self.IsDense?` false))
    (:`4`
      (`StaticMeshComponent.SetStaticMesh` (`self.StaticMesh`) (`self.FloorSM`))
      (bind _returnvalue_4 (`PrimitiveComponent.CreateDynamicMaterialInstance` (`self.StaticMesh`) 0 "/Game/StarterContent/Materials/M_Ceramic_Tile_Checker.M_Ceramic_Tile_Checker" "None"))
      (set `self.MaterialInstance` _returnvalue_4)
      (goto _label))
    (:`5`
      (`StaticMeshComponent.SetStaticMesh` (`self.StaticMesh`) (`self.WallSM`))
      (bind _returnvalue_5 (`PrimitiveComponent.CreateDynamicMaterialInstance` (`self.StaticMesh`) 0 "/Game/Materials/MI_Walltile.MI_Walltile" "None"))
      (set `self.MaterialInstance` _returnvalue_5)
      (set `self.isInSpace?` false)
      (set `self.IsDense?` true))))

(fn `UpdateAirHUD`
  (bind _asatmos_hud (cast `/Game/Blueprints/Turf/Atmos_HUD` (`WidgetComponent.GetUserWidgetObject` (`self.Widget`))))
  (`/Game/Blueprints/Turf/Atmos_HUD.UpdateAir` _asatmos_hud (`KismetMathLibrary.Conv_IntToDouble` (`self.Oxygen`)) (`KismetMathLibrary.Conv_IntToDouble` (`self.Nitrogen`)) (`KismetMathLibrary.Conv_IntToDouble` (`self.CarbonDioxide`)) (`KismetMathLibrary.Conv_IntToDouble` (`self.Temperature`)) (`KismetMathLibrary.Conv_IntToDouble` (`self.Pressure`))))

(fn `UserConstructionScript`
  (`parent.UserConstructionScript`)
  (`self.SetTileType` (`self.TurfType`))
  (`self.DefaultAir`)
  (`self.UpdateAirHUD`))