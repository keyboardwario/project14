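; BP_TileMap is the grid map actor that generates and owns the Turf tiles of a level.
; ResetMap destroys all BP_Atom actors, spawns and attaches turfs across a Width by Height grid, then has them discover neighbors and open-air links.
; Turf types come from a seeded, clamped random walk despite the Perlin name, with border tiles forced to zero.
; Helpers handle tile lookup and chunk saving through LevelChunkSave; UpdateAir is an empty stub.
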(event `Event UpdateAir`
  (for _ (`self.Turfs`)
    _))

(fn `FindUnoccupiedTurf`
  (returns (Unoccupied :type "/Game/Blueprints/Turf/Turf Object Reference"))
  (locals (UnoccupiedTurf :type "/Game/Blueprints/Turf/Turf Object Reference"))
  (bind _turfs (`self.Turfs`))
  (for _array_element _turfs
    (if (== (`/Game/Blueprints/Turf/Turf.TurfType` _array_element) 4)
      (set `local.UnoccupiedTurf` _array_element)
      (break)))
  (bind _unoccupiedturf (`local.UnoccupiedTurf`)
    (:`then`
      (return _unoccupiedturf))
    (:`else`
      (bind _output_get (set `local.UnoccupiedTurf` (`|GetArrayItem` _turfs)))
      (return _output_get))))

(fn `GetTurfAtCoord`
  (params (coord :type "/Game/Library/Coord Structure"))
  (returns (turf :type "/Game/Blueprints/Turf/Turf Object Reference"))
  (return (`|GetArrayItem` (`self.Turfs`) (`/Game/Library/GridMath.CoordToIndex` self coord))))

(fn `Index To Location`
  (params (Index :type Integer) (`Center?` :type Boolean))
  (returns (`Valid?` :type Boolean) (Location :type "Vector2D Structure"))
  (bind _tile_size (`self.Tile Size`))
  (bind _tile_size_2 (`self.Tile Size`))
  (bind _tile_size_3 (`self.Tile Size`))
  (if (`KismetMathLibrary.InRange_IntInt` Index 0 (`self.Total Tiles -1`))
    (if `Center?`
      (return true (`KismetMathLibrary.MakeVector2D` (+ (/ _tile_size 2.0) (* (mod Index (`self.Width`)) _tile_size_2)) (+ (/ _tile_size 2.0) (* (/ Index (`self.Height`)) _tile_size_2))))
      (else
        (return true (`KismetMathLibrary.MakeVector2D` (* (mod Index (`self.Width`)) _tile_size_3) (* (/ Index (`self.Height`)) _tile_size_3)))))
    (else
      (return false (0.0 0.0)))))

(fn `IsCoordOnBorder`
  (params (Index :type Integer))
  (returns (ReturnValue :type Boolean))
  (bind _coord (`/Game/Library/GridMath.IndexToCoord` Index self))
  (return (or (== (break `/Game/Library/Coord` _coord) (- (`self.Width`) 1)) (== (`.Y_5_639F436E4C84DCC6574B3BA4527F0F32` (break `/Game/Library/Coord` _coord)) (- (`self.Height`) 1)) (== (break `/Game/Library/Coord` _coord) 0) (== (`.Y_5_639F436E4C84DCC6574B3BA4527F0F32` (break `/Game/Library/Coord` _coord)) 0))))

(fn `LoadChunk`
  (params (SlotName :type String))
  (bind _returnvalue (`GameplayStatics.DoesSaveGameExist` SlotName))
  (if _returnvalue
    (bind _returnvalue_2 (`GameplayStatics.LoadGameFromSlot` SlotName))
    (bind _aslevel_chunk_save (cast `/Game/Library/LevelChunkSave` _returnvalue_2))
    (set `self.ChunkBeingSaved` _aslevel_chunk_save)
    (else
      (bind _returnvalue_3 (`GameplayStatics.CreateSaveGameObject` "/Game/Library/LevelChunkSave.LevelChunkSave_C"))
      (set `self.ChunkBeingSaved` _returnvalue_3))))

(fn `PerlinTilesTEMP`
  (returns (`RandomPerlin (0-5)` :type Integer))
  (bind _temprandom (`self.TempRandom`))
  (switch `int` (`KismetMathLibrary.RandomIntegerInRangeFromStream` 0 2 (`self.Seed`))
    (:`0`
      (`/Engine/EditorBlueprintResources/StandardMacros.IncrementInt` _temprandom
        (:`  `
          _)))
    (:`1`
      _)
    (:`2`
      (`/Engine/EditorBlueprintResources/StandardMacros.DecrementInt` _temprandom
        (:`  `
          _))))
  (bind _output_get (set `self.TempRandom` (`KismetMathLibrary.Clamp` (`self.TempRandom`) 0 5)))
  (return _output_get))

(fn `ResetMap`
  (bind _box (`self.Box`))
  (bind _height (`self.Height`))
  (bind _tile_size (`self.Tile Size`))
  (bind _width (`self.Width`))
  (bind _tile_size_2 (`self.Tile Size`))
  (bind _returnvalue (/ (* (`self.Height`) _tile_size) 2.0))
  (bind _returnvalue_2 (/ (* (`self.Width`) _tile_size) 2.0))
  (set `self.Timer` (`GameplayStatics.GetWorldDeltaSeconds`))
  (`|ExecutionSequence`
    (:`then_0`
      ;[1 1 1] Clean up
      (bind _outactors (`GameplayStatics.GetAllActorsOfClass` "/Game/Blueprints/Atom/BP_Atom.BP_Atom_C"))
      (for _array_element _outactors
        (`self.K2_DestroyActor` _array_element))
      (`KismetArrayLibrary.Array_Clear` (`self.Turfs`))
      (`BlueprintMapLibrary.Map_Clear` (`self.TileIndexCoord`)))
    (:`then_1`
      ;[1 1 1] Resize Arrays all at once - this way I can use set array elem instead of Add, I think its faster?
      (`KismetArrayLibrary.Array_Resize` (`self.Turfs`) (* (`self.Height`) (`self.Width`))))
    (:`then_2`
      (bind (_current_point _total_points _0_1_phase _poly_center _x_row _y_row) (`/Engine/ArtTools/RenderToTexture/Macros/RenderToTextureMacros.2D Grid Execution Macro` _tile_size_2 (`KismetMathLibrary.MakeVector` (/ (* _width _tile_size_2) 2.0) (/ (* _height _tile_size_2) 2.0)) _width _height)
        (:`Per Poly Execution`
          (bind _returnvalue_3 (`self.IsCoordOnBorder` _current_point))
          (if _returnvalue_3
            (set `self.TempRandom` 0)
            (else
              (`self.PerlinTilesTEMP`)))
          (bind _returnvalue_4 (`|SpawnActorFromClass` "/Game/Blueprints/Turf/Turf.Turf_C" (`KismetMathLibrary.MakeTransform` _poly_center) "AlwaysSpawn" "OverrideRootScale" null _current_point (`self.TempRandom`) (make `/Game/Library/Coord` _x_row _y_row) self null null))
          (`KismetArrayLibrary.Array_Set` (`self.Turfs`) _current_point _returnvalue_4)
          (`self.K2_AttachToActor` _returnvalue_4 self "None" "KeepWorld" "KeepWorld" "KeepWorld" true) ; this is just so i can collapse it in editor
        )))
    (:`then_3`
      ;[1 1 1] Turfs Find Neighbor Turfs and Map Them to Directions & Map Open Air Neighbors for indoor tiles
      (for _array_element_2 (`self.Turfs`)
        (`/Game/Blueprints/Turf/Turf.DiscoverNeighborTiles` _array_element_2)))
    (:`then_4`
      ;[1 1 1] debug box around the map
      (`SceneComponent.K2_SetWorldLocation` _box (`KismetMathLibrary.MakeVector` _returnvalue_2 _returnvalue) false true)
      (`BoxComponent.SetBoxExtent` _box (`KismetMathLibrary.MakeVector` _returnvalue_2 _returnvalue) true))
    (:`then_5`
      (for _array_element_3 (`self.Turfs`)
        (`/Game/Blueprints/Turf/Turf.FindOpenAirNeighbors` _array_element_3)))))

(fn `SaveChunk`
  (params (Width :type Integer) (Height :type Integer) (TurfTypeArray :type "Array of Integer") (`Save Name` :type String))
  (returns (`SaveSuccess?` :type Boolean))
  (`|ExecutionSequence`
    (:`then_0`
      (`self.LoadChunk` `Save Name`))
    (:`then_1`
      (bind _chunkbeingsaved (`self.ChunkBeingSaved`)
        (:`then`
          (set `/Game/Library/LevelChunkSave.BasicSetupInfo` (make `/Game/Library/LevelChunk` Width Height TurfTypeArray) _chunkbeingsaved))
        (:`else`)))
    (:`then_2`
      (bind _returnvalue (`GameplayStatics.SaveGameToSlot` (`self.ChunkBeingSaved`) `Save Name`))
      (return _returnvalue))))

(fn `UserConstructionScript`)